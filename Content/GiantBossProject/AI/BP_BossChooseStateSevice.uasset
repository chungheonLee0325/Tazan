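; Behavior tree service that picks the giant boss's state from its distance to the player.
; Each tick it measures the gap between the controlled pawn and player pawn 0, then writes one of three enum values to a blackboard key.
; A fixed cutoff selects the far state, while a randomized threshold rolled on every evaluation splits close from mid range, making that boundary unpredictable.
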(event `self.ReceiveTickAI`
  (params (OwnerController :type "AIController Object Reference") (ControlledPawn :type "Pawn Object Reference") (DeltaSeconds :type "Float (single-precision)"))
  (bind _returnvalue (`AIBlueprintHelperLibrary.GetBlackboard` ControlledPawn))
  (bind _keyname (`self.KeyName`))
  (bind _returnvalue_2 (`KismetMathLibrary.VSize` (- (`Actor.K2_GetActorLocation` ControlledPawn) (`Actor.K2_GetActorLocation` (`GameplayStatics.GetPlayerPawn` 0)))))
  (if (>= _returnvalue_2 3000.0)
    (`BlackboardComponent.SetValueAsEnum` _returnvalue _keyname 0)
    (elif (<= _returnvalue_2 (`KismetMathLibrary.RandomFloatInRange` 200.0 1000.0))
      (`BlackboardComponent.SetValueAsEnum` _returnvalue _keyname 2)
      (else
        (`BlackboardComponent.SetValueAsEnum` _returnvalue _keyname 1)))))