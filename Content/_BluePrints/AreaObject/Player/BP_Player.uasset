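; Player character Blueprint whose event graph holds only debug hotkeys and leftover test nodes.
; Key 3 feeds a strong-stagger hit with hit stop into MPoiseComponent.
; Key 2 calls ExchangeDead on MConditionComponent and runs OnDie if it returns true.
; Disconnected experiments for montages, skills, camera rotation, sound, damage and weapon-socket traces never run; BeginPlay, Tick and the construction script are empty.
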(event `self.ReceiveBeginPlay`)

(event `self.ReceiveTick`
  (params (DeltaSeconds :type "Float (single-precision)")))

(event `Key|Three`
  (params (Key :type "Key Structure"))
  (:`Pressed`
    (`PoiseComponent.PoiseProcess` (`self.m_PoiseComponent`) (make `AttackData` 1.0 1.0 3.0 4 "Strong" (struct :`DetectionType` "Line" :`Radius` 15.0 :`HalfHeight` 30.0 :`BoxExtent` (15.0 15.0 15.0) :`InterpolationSteps` 4) true 3.0) (`self.Direction`))))

(event `Key|Two`
  (params (Key :type "Key Structure"))
  (:`Pressed`
    (bind _returnvalue (`ConditionComponent.ExchangeDead` (`self.m_ConditionComponent`)))
    (if _returnvalue
      (`self.OnDie`))))

(event `Key|Four`
  (params (Key :type "Key Structure")))

(fn `UserConstructionScript`)